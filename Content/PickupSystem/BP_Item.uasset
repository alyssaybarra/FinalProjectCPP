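; BP_Item is a pickup actor whose static mesh is chosen through the ItemModelToPlace variable and applied in the construction script.
; Its Pickup event prints a debug message and plays a timeline that scales the root from full size toward zero.
; The sound and delayed destroy hang off the timeline's Update, so the 2D pickup sound fires on every update until the actor is destroyed.
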(event EventBeginPlay)

(event Collision|EventActorBeginOverlap
  (params (OtherActor :type Actor%20Object%20Reference)))

(event EventTick
  (params (DeltaSeconds :type Float%20%28single-precision%29)))

(event EventPickup
  (Development|PrintString "Item Picked")
  (bind _shinktimeline (Timeline|Shrink Play)
    (:Update
      (Transformation|SetWorldScale3D (Variables|Default|GetDefaultSceneRoot) (Math|Conversions|ToVector(Float) (Math|Float|Lerp 1.0 0.0 _shinktimeline)))
      (Audio|PlaySound2D "/Game/563465__nicholasdaryl__itempickup.563465__nicholasdaryl__itempickup" 1.0 1.0 0.0 0 0)
      (Utilities|FlowControl|Delay 0.4)
      (Actor|DestroyActor))))

(fn ConstructionScript
  (Components|StaticMesh|SetStaticMesh (Variables|Default|GetItemModel) (Variables|Default|GetItemModelToPlace)))